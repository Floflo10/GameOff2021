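; BP_Pawn is a pawn that moves its Camera from player input, apparently for viewing in the DNA project.
; MoveRight, MoveForward and mouse wheel axes add local offsets on Z, Y and X respectively, scaled by Acceleration.
; Each input applies only while the Move flag on the DNA_Controler player controller is true.
; Movement is per input event, with no delta-time scaling visible.
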(event `InputAxis|MoveRight`
  (params (AxisValue :type "Float (single-precision)"))
  (if (`/Game/DNA/Core/DNA_Controler.Move?` (cast `/Game/DNA/Core/DNA_Controler` (`GameplayStatics.GetPlayerController` 0) :!pure true))
    (bind _result (`/Engine/EditorBlueprintResources/StandardMacros.NegateFloat` AxisValue)
      (:`  `
        (`SceneComponent.K2_AddLocalOffset` (`self.Camera`) (`KismetMathLibrary.MakeVector` 0.0 0.0 (* _result (`self.Acceleration`))) false false)))))

(event `InputAxis|MoveForward`
  (params (AxisValue :type "Float (single-precision)"))
  (if (`/Game/DNA/Core/DNA_Controler.Move?` (cast `/Game/DNA/Core/DNA_Controler` (`GameplayStatics.GetPlayerController` 0) :!pure true))
    (bind _result (`/Engine/EditorBlueprintResources/StandardMacros.NegateFloat` AxisValue)
      (:`  `
        (`SceneComponent.K2_AddLocalOffset` (`self.Camera`) (`KismetMathLibrary.MakeVector` 0.0 (* _result (`self.Acceleration`))) false false)))))

(event `InputAxisKey|MouseWheelAxis`
  (params (AxisValue :type "Float (single-precision)"))
  (if (`/Game/DNA/Core/DNA_Controler.Move?` (cast `/Game/DNA/Core/DNA_Controler` (`GameplayStatics.GetPlayerController` 0) :!pure true))
    (`SceneComponent.K2_AddLocalOffset` (`self.Camera`) (`KismetMathLibrary.MakeVector` (* AxisValue (`self.Acceleration`))) false false)))

(fn `UserConstructionScript`)