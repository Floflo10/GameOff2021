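; Blood manager actor that simulates the body's protein stock and random protein demands, ending the game when unknown proteins corrupt the blood.
; StockProtein resolves formulas through DT_Protein into an array and a per-name count map.
; Each DNA_Mode pulse ages and expires proteins, spends Macrophages against unknowns, updates needs on WBP_InteractionScreen and checks integrity.
; An exactly met need triggers another request; the RandomAskProt timer only runs a delay.
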(event `self.ReceiveBeginPlay`
  (add `/Game/DNA/Core/DNA_Mode.Pulse` (cast `/Game/DNA/Core/DNA_Mode` (`GameplayStatics.GetGameMode`) :!pure true) (delegate `PulseEvent`))
  (`KismetSystemLibrary.Delay` 0.2)
  (bind _foundwidgets (`WidgetBlueprintLibrary.GetAllWidgetsOfClass` "/Game/DNA/Core/Widget/WBP_InteractionScreen.WBP_InteractionScreen_C" false))
  (set `self.InteractionWidget` (`|GetArrayItem` _foundwidgets))
  (`KismetSystemLibrary.K2_SetTimerDelegate` (delegate `RandomAskProt`) 4.0 true)
  (`self.AskForProtein`)
  (while (> (`self.Charge`) 1)
    (`self.StockProtein` "147857478")
    (`/Engine/EditorBlueprintResources/StandardMacros.DecrementInt` (`self.Charge`))))

(event `PulseEvent`
  (`self.DecreaseProt`)
  (`self.KillProtein`)
  (`self.ConsumProtein`)
  (`self.CheckIfCorrupted`))

(event `RandomAskProt`
  (`KismetSystemLibrary.Delay` (`KismetMathLibrary.RandomFloatInRange` 10.0 (`self.MaxTimeBeforeAsk`))))

(event `StockProtein`
  (params (Formule :type String))
  (bind _proteinnumberinblood (`self.ProteinNumberInBlood`))
  (bind _proteininblood (`self.ProteinInBlood`))
  (bind (_output_formule _output_nom) (break `/Game/DNA/Core/Gameplay/SProtein` (`|GetArrayItem` _proteininblood (`KismetArrayLibrary.Array_LastIndex` _proteininblood))))
  (bind (_value _returnvalue) (`BlueprintMapLibrary.Map_Find` _proteinnumberinblood _output_nom))
  (bind _returnvalue_2 (`|GetDataTableRow` "/Game/DNA/Core/Gameplay/DT_Protein.DT_Protein" (`KismetStringLibrary.Conv_StringToName` Formule))
    (:`then`
      (bind _returnvalue_3 (`KismetArrayLibrary.Array_Add` (`self.ProteinInBlood`) _returnvalue_2))
      (`KismetSystemLibrary.PrintString` (`KismetStringLibrary.Concat_StrStr` "Tab Number  " (`KismetStringLibrary.Conv_IntToString` _returnvalue_3))))
    (:`RowNotFound`
      (bind _returnvalue_4 (`KismetArrayLibrary.Array_Add` _proteininblood (make `/Game/DNA/Core/Gameplay/SProtein` (`KismetStringLibrary.Conv_StringToInt` Formule) "Unknow Protein" null 9999)))
      (`KismetSystemLibrary.PrintString` (`KismetStringLibrary.Concat_StrStr` "Tab Number  " (`KismetStringLibrary.Conv_IntToString` _returnvalue_4)))))
  (if _returnvalue
    (bind _result (`/Engine/EditorBlueprintResources/StandardMacros.IncrementInt` _value)
      (:`  `
        (`BlueprintMapLibrary.Map_Add` _proteinnumberinblood _output_nom _result)
        (`KismetSystemLibrary.PrintString` (`KismetStringLibrary.Conv_IntToString` (`BlueprintMapLibrary.Map_Find` _proteinnumberinblood _output_nom)))))
    (else
      (`BlueprintMapLibrary.Map_Add` _proteinnumberinblood _output_nom 1))))

(event `CheckIfCorrupted`
  (bind _returnvalue (- 100 (* (/ (`KismetMathLibrary.Conv_IntToDouble` (`BlueprintMapLibrary.Map_Find` (`self.ProteinNumberInBlood`) "Unknow Protein")) (`KismetMathLibrary.Conv_IntToDouble` (`KismetArrayLibrary.Array_Length` (`self.ProteinInBlood`)))) 100.0)))
  (set `self.BodyIntegrity` _returnvalue)
  (if (< _returnvalue (`/Game/DNA/Core/DNA_Mode.LimiteUnknow` (cast `/Game/DNA/Core/DNA_Mode` (`GameplayStatics.GetGameMode`) :!pure true)))
    (`/Game/DNA/Core/DNA_Mode.EndGame` (cast `/Game/DNA/Core/DNA_Mode` (`GameplayStatics.GetGameMode`) :!pure true))))

(event `KillProtein`
  (bind _proteininblood (`self.ProteinInBlood`))
  (bind _proteinnumberinblood (`self.ProteinNumberInBlood`))
  (bind _proteininblood_2 (`self.ProteinInBlood`))
  (bind _proteinnumberinblood_2 (`self.ProteinNumberInBlood`))
  (bind _proteinnumberinblood_3 (`self.ProteinNumberInBlood`))
  (for (_array_element _array_index) _proteininblood_2
    (bind _output_get (set `self.TempProtein` _array_element))
    (`|ExecutionSequence`
      (:`then_0`
        (if (<= (`.PulseLifeCycle_9_EF90FAEE45E2569A56F4978829BEF444` (break `/Game/DNA/Core/Gameplay/SProtein` _output_get)) 0)
          (`KismetArrayLibrary.Array_Remove` _proteininblood_2 _array_index)
          (bind _result (`/Engine/EditorBlueprintResources/StandardMacros.DecrementInt` (`BlueprintMapLibrary.Map_Find` _proteinnumberinblood_2 (`.Nom_6_F3C106F04B262DEAB109BB984ECD5D11` (break `/Game/DNA/Core/Gameplay/SProtein` _output_get))))
            (:`  `
              (if (<= _result 0)
                (`BlueprintMapLibrary.Map_Remove` _proteinnumberinblood_2 (`.Nom_6_F3C106F04B262DEAB109BB984ECD5D11` (break `/Game/DNA/Core/Gameplay/SProtein` _output_get)))
                (else
                  (`BlueprintMapLibrary.Map_Add` _proteinnumberinblood_2 (`.Nom_6_F3C106F04B262DEAB109BB984ECD5D11` (break `/Game/DNA/Core/Gameplay/SProtein` _output_get)) _result)))))))
      (:`then_1`
        (if (and (== (`.Nom_6_F3C106F04B262DEAB109BB984ECD5D11` (break `/Game/DNA/Core/Gameplay/SProtein` _output_get)) "Unknow Protein") (> (`self.MacrophageNumber`) 0))
          (`KismetArrayLibrary.Array_Remove` _proteininblood_2 _array_index)
          (bind _result_2 (`/Engine/EditorBlueprintResources/StandardMacros.DecrementInt` (`BlueprintMapLibrary.Map_Find` _proteinnumberinblood_3 (`.Nom_6_F3C106F04B262DEAB109BB984ECD5D11` (break `/Game/DNA/Core/Gameplay/SProtein` _output_get))))
            (:`  `
              (if (== _result_2 0)
                (`BlueprintMapLibrary.Map_Remove` _proteinnumberinblood_3 (`.Nom_6_F3C106F04B262DEAB109BB984ECD5D11` (break `/Game/DNA/Core/Gameplay/SProtein` _output_get)))
                (else
                  (`BlueprintMapLibrary.Map_Add` _proteinnumberinblood_3 (`.Nom_6_F3C106F04B262DEAB109BB984ECD5D11` (break `/Game/DNA/Core/Gameplay/SProtein` _output_get)) _result_2)))
              (for (_array_element_2 _array_index_2) _proteininblood
                (bind _output_get_2 (set `self.TempProtein` _array_element_2))
                (if (== (`.Nom_6_F3C106F04B262DEAB109BB984ECD5D11` (break `/Game/DNA/Core/Gameplay/SProtein` _output_get_2)) "Macrophage")
                  (`KismetArrayLibrary.Array_Remove` _proteininblood _array_index_2)
                  (bind _result_3 (`/Engine/EditorBlueprintResources/StandardMacros.DecrementInt` (`BlueprintMapLibrary.Map_Find` _proteinnumberinblood (`.Nom_6_F3C106F04B262DEAB109BB984ECD5D11` (break `/Game/DNA/Core/Gameplay/SProtein` _output_get_2))))
                    (:`  `
                      (if (== _result_3 0)
                        (`BlueprintMapLibrary.Map_Remove` _proteinnumberinblood (`.Nom_6_F3C106F04B262DEAB109BB984ECD5D11` (break `/Game/DNA/Core/Gameplay/SProtein` _output_get_2)))
                        (break)
                        (else
                          (`BlueprintMapLibrary.Map_Add` _proteinnumberinblood (`.Nom_6_F3C106F04B262DEAB109BB984ECD5D11` (break `/Game/DNA/Core/Gameplay/SProtein` _output_get_2)) _result_3)
                          (break))))))))))))))

(event `AskForProtein`
  (bind _proteinaskedinblood (`self.ProteinAskedInBlood`))
  (bind _randomprotein (`self.RandomProtein`))
  (bind _returnvalue (* (`KismetMathLibrary.RandomIntegerInRange` 1 14) 2))
  (while (or (== _randomprotein "147857478") (== _randomprotein ""))
    (bind _returnvalue_2 (`DataTableFunctionLibrary.GetDataTableColumnAsString` "/Game/DNA/Core/Gameplay/DT_Protein.DT_Protein" "Formule"))
    (set `self.RandomProtein` (`KismetArrayLibrary.Array_Random` _returnvalue_2)))
  (bind _returnvalue_3 (`|GetDataTableRow` "/Game/DNA/Core/Gameplay/DT_Protein.DT_Protein" (`KismetStringLibrary.Conv_StringToName` (`self.RandomProtein`)))
    (:`then`
      (bind (_value _returnvalue_4) (`BlueprintMapLibrary.Map_Find` _proteinaskedinblood (`.Nom_6_F3C106F04B262DEAB109BB984ECD5D11` (break `/Game/DNA/Core/Gameplay/SProtein` _returnvalue_3))))
      (if _returnvalue_4
        (`BlueprintMapLibrary.Map_Add` _proteinaskedinblood (`.Nom_6_F3C106F04B262DEAB109BB984ECD5D11` (break `/Game/DNA/Core/Gameplay/SProtein` _returnvalue_3)) (+ _value _returnvalue))
        (set `self.RandomProtein` "")
        (else
          (`BlueprintMapLibrary.Map_Add` _proteinaskedinblood (`.Nom_6_F3C106F04B262DEAB109BB984ECD5D11` (break `/Game/DNA/Core/Gameplay/SProtein` _returnvalue_3)) _returnvalue)
          (set `self.RandomProtein` "" :!label _label))))
    (:`RowNotFound`
      (goto _label))))

(event `ConsumProtein`
  (bind _proteinaskedinblood (`self.ProteinAskedInBlood`))
  (bind _keys (`BlueprintMapLibrary.Map_Keys` _proteinaskedinblood))
  (for _array_element _keys
    (bind _value (`BlueprintMapLibrary.Map_Find` (`self.ProteinNumberInBlood`) _array_element))
    (bind _value_2 (`BlueprintMapLibrary.Map_Find` _proteinaskedinblood _array_element))
    (if (!= _value _value_2)
      (`/Game/DNA/Core/Widget/WBP_InteractionScreen.Add Need` (`self.InteractionWidget`) _array_element (`KismetTextLibrary.Conv_NameToText` _array_element) (`KismetTextLibrary.Conv_StringToText` (`KismetStringLibrary.Concat_StrStr` (`KismetStringLibrary.Conv_IntToString` _value) " / " (`KismetStringLibrary.Conv_IntToString` _value_2))))
      (else
        (`/Game/DNA/Core/Widget/WBP_InteractionScreen.Delete Need` (`self.InteractionWidget`) _array_element "" "")
        (`self.AskForProtein`))))
  (set `self.MacrophageNumber` (`BlueprintMapLibrary.Map_Find` (`self.ProteinNumberInBlood`) "Macrophage")))

(event `DecreaseProt`
  (bind _proteininblood (`self.ProteinInBlood`))
  (for (_array_element _array_index) (`self.ProteinInBlood`)
    (`KismetArrayLibrary.Array_Set` _proteininblood _array_index (make `/Game/DNA/Core/Gameplay/SProtein` (break `/Game/DNA/Core/Gameplay/SProtein` _array_element) (`.Nom_6_F3C106F04B262DEAB109BB984ECD5D11` (break `/Game/DNA/Core/Gameplay/SProtein` _array_element)) (`.LinkedParticule_14_5C47F937479EFBF4C2EA4C9FEAF972B4` (break `/Game/DNA/Core/Gameplay/SProtein` _array_element)) (- (`.PulseLifeCycle_9_EF90FAEE45E2569A56F4978829BEF444` (break `/Game/DNA/Core/Gameplay/SProtein` _array_element)) 1)))
    (bind (_output_formule _output_nom _output_linkedparticule _output_pulselifecycle) (break `/Game/DNA/Core/Gameplay/SProtein` (`|GetArrayItem` _proteininblood _array_index)))
    (`KismetSystemLibrary.PrintString` (`KismetStringLibrary.Conv_IntToString` _output_pulselifecycle))))

(fn `UserConstructionScript`)