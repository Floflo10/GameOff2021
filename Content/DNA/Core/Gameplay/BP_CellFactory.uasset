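; Cell factory actor that produces protein code strings on each game-mode pulse and passes them to linked factories.
; Each pulse appends its protein to the incoming string, pushes it downstream and optionally stocks it in BloodManager, triggering Niagara particles driven by DT_Protein.
; Random mutation, likelier with more links, randomizes the protein and forces blood export until it matches the chosen one.
; Cable components show links, and cell scale grows with link count.
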(event `self.ReceiveBeginPlay`
  (add `/Game/DNA/Core/DNA_Mode.Pulse` (cast `/Game/DNA/Core/DNA_Mode` (`GameplayStatics.GetGameMode`) :!pure true) (delegate `PulseEvent`))
  (bind _outactors (`GameplayStatics.GetAllActorsOfClass` "/Game/DNA/Core/Gameplay/BP_BloodManager.BP_BloodManager_C"))
  (set `self.BloodManager` (`|GetArrayItem` _outactors)))

(event `PulseEvent`
  (`self.CheckPulse`)
  (`self.CheckEntry`)
  (`self.SendProteinToCell`)
  (`self.SendToBlood`)
  (`self.IsMuting?`)
  (`self.CheckMutation`)
  (`self.SetSize`))

(event `CheckPulse`
  (`/Engine/EditorBlueprintResources/StandardMacros.IncrementInt` (`self.ActualPulse`)
    (:`  `
      (if (== (`self.MaxPulse`) (`self.ActualPulse`))
        (set `self.ActualPulse` 0)))))

(event `SendProteinToCell`
  (for _array_element (`self.Connected Factory`)
    (set `/Game/DNA/Core/Gameplay/BP_CellFactory.EntryPoint` (`self.NextExport`) _array_element)))

(event `CheckEntry`
  (if (> (`KismetStringLibrary.Conv_StringToInt` (`self.EntryPoint`)) 0)
    (set `self.NextExport` (`KismetStringLibrary.Concat_StrStr` (`self.EntryPoint`) (`self.ProteineProducted`)))
    (else
      (set `self.NextExport` (`self.ProteineProducted`)))))

(event `CheckMutation`
  (if (`|EnumEquality` (`self.CellState`) "NewEnumerator1")
    (`PrimitiveComponent.SetMaterial` (`self.Cell`) 0 "/Game/DNA/Core/Material/M_CircleMutation.M_CircleMutation")
    (set `self.SendToBlood?` true)
    (if (== (`self.ProteineProducted`) (`self.ProteineChosen`))
      (set `self.CellState` "NewEnumerator0")
      (`PrimitiveComponent.SetMaterial` (`self.Cell`) 0 "/Game/DNA/Core/Material/M_CircleOk.M_CircleOk"))))

(event `IsMuting?`
  (if (== (`KismetMathLibrary.RandomIntegerInRange` 0 (/ (`self.Max`) (+ (`KismetArrayLibrary.Array_Length` (`self.Connected Factory`)) 1 (`self.SendToBlood?`)))) 1)
    (set `self.CellState` "NewEnumerator1")
    (set `self.ProteineProducted` (`KismetStringLibrary.Conv_IntToString` (`KismetMathLibrary.RandomIntegerInRange` 0 9)))))

(event `SpawnPart`
  (bind _niagara (`self.Niagara`))
  (bind _nextexport (`self.NextExport`))
  (switch `/Game/DNA/Core/Gameplay/ECellState` (`self.CellState`)
    (:`NewEnumerator0`
      (if (== (`self.NextExport`) "147857478")
        (set `self.ColorPart` (struct :`G` 142.427444 :`B` 200.0 :`A` 1.0))
        (`NiagaraComponent.SetVariableLinearColor` _niagara "User.color" (`self.ColorPart`))
        (else
          (set `self.ColorPart` (struct :`R` 150.0 :`G` 140.0 :`B` 150.0 :`A` 1.0))
          (`NiagaraComponent.SetVariableLinearColor` _niagara "User.color" (`self.ColorPart`)))))
    (:`NewEnumerator1`
      (set `self.ColorPart` (struct :`R` 23.985386 :`B` 250.0 :`A` 1.0))
      (`NiagaraComponent.SetVariableLinearColor` _niagara "User.Color" (`self.ColorPart`))))
  (bind _returnvalue (`|GetDataTableRow` "/Game/DNA/Core/Gameplay/DT_Protein.DT_Protein" (`KismetStringLibrary.Conv_StringToName` _nextexport))
    (:`then`
      (`NiagaraComponent.SetVariableFloat` _niagara "User.Lifetime" (`KismetMathLibrary.Conv_IntToDouble` (`.PulseLifeCycle_9_EF90FAEE45E2569A56F4978829BEF444` (break `/Game/DNA/Core/Gameplay/SProtein` _returnvalue)))))
    (:`RowNotFound`
      (`NiagaraComponent.SetVariableFloat` _niagara "User.Lifetime" 9999.0)))
  (`NiagaraComponent.SetVariableFloat` _niagara "User.Number" (`KismetMathLibrary.Conv_IntToDouble` (`KismetStringLibrary.Len` _nextexport)))
  (`ActorComponent.Activate` _niagara true))

(event `ConnectCell`
  (params (DestinationCell :type "/Game/DNA/Core/Gameplay/BP_CellFactory Object Reference"))
  (`KismetArrayLibrary.Array_AddUnique` (`self.Connected Factory`) DestinationCell)
  (set `/Game/DNA/Core/Gameplay/BP_CellFactory.EntryPoint` (`self.NextExport`) DestinationCell)
  (`KismetSystemLibrary.PrintString` (`KismetStringLibrary.Concat_StrStr` (`KismetSystemLibrary.GetDisplayName` self) "Link to " (`KismetSystemLibrary.GetDisplayName` DestinationCell)) true true (struct :`R` 0.867051 :`G` 1.0 :`A` 1.0) 5.0)
  (bind _returnvalue (`AddComponent|NODE_AddCableComponent-0` :`bManualAttachment` true :`RelativeTransform` (`SceneComponent.K2_GetComponentToWorld` (`self.Box`))))
  (`BlueprintMapLibrary.Map_Add` (`self.Cable Factory`) DestinationCell _returnvalue)
  (`BlueprintMapLibrary.Map_Add` (`/Game/DNA/Core/Gameplay/BP_CellFactory.Cable Factory` DestinationCell) self _returnvalue)
  (`CableComponent.SetAttachEndTo` _returnvalue DestinationCell "None" "None"))

(event `Selected`
  (`PrimitiveComponent.SetMaterial` (`self.Cell`) 0 "/Game/DNA/Core/Material/M_CircleSelect.M_CircleSelect"))

(event `self.ReceiveDestroyed`
  (bind _entrycell (`self.EntryCell`))
  (for _array_element (`self.Connected Factory`)
    (set `/Game/DNA/Core/Gameplay/BP_CellFactory.EntryCell` null _array_element))
  (if (!= _entrycell null)
    (`self.DestroyLink` _entrycell self)))

(event `Unselect`
  (`PrimitiveComponent.SetMaterial` (`self.Cell`) 0 "/Game/DNA/Core/Material/M_CircleOk.M_CircleOk"))

(event `SetEntryPoint`
  (params (EntryCell :type "/Game/DNA/Core/Gameplay/BP_CellFactory Object Reference"))
  (bind _output_get (set `self.EntryCell` EntryCell))
  (set `self.EntryPoint` (`/Game/DNA/Core/Gameplay/BP_CellFactory.NextExport` _output_get)))

(event `DestroyLink`
  (params (CHild :type "/Game/DNA/Core/Gameplay/BP_CellFactory Object Reference"))
  (bind _cable_factory (`self.Cable Factory`))
  (`ActorComponent.K2_DestroyComponent` (`BlueprintMapLibrary.Map_Find` _cable_factory CHild))
  (`BlueprintMapLibrary.Map_Remove` _cable_factory CHild))

(event `Setting`
  (set `self.ProteineChosen` (`self.ProteineProducted`)))

(event `SendToBlood`
  (if (`self.SendToBlood?`)
    (`/Game/DNA/Core/Gameplay/BP_BloodManager.StockProtein` (`self.BloodManager`) (`self.NextExport`))
    (`self.SpawnPart`)))

(event `SetSize`
  (`SceneComponent.SetRelativeScale3D` (`self.Cell`) (+ (`KismetMathLibrary.Conv_DoubleToVector` (* (`KismetArrayLibrary.Array_Length` (`self.Connected Factory`)) 0.1)) (0.5 0.5 0.5))))

(fn `UserConstructionScript`)